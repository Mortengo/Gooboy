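; BP_Enemy is an enemy actor with health and a health bar widget component.
; On BeginPlay it passes itself to its BP_EnemyHealthUI widget, then initializes current health and percent.
; GenerateDamage subtracts damage, destroys the actor when health runs out, and otherwise recalculates health percent on a 0–100 scale.
; It never pushes that percent to the widget, as the SetPercent call is disconnected; debug prints report the values.
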(event `self.ReceiveBeginPlay`
  (bind _asbp_enemy_health_ui (cast `/Game/Blueprints/BP_EnemyHealthUI` (`WidgetComponent.GetUserWidgetObject` (`self.HealthBar`))))
  (set `/Game/Blueprints/BP_EnemyHealthUI.Enemy` self _asbp_enemy_health_ui)
  (bind _output_get (set `self.CurrentHealth` (`self.InitialHealth`)))
  (bind _output_get_2 (set `self.CurrentPercent` (`self.InitialPercent`)))
  (`KismetSystemLibrary.PrintString` (`KismetStringLibrary.Conv_IntToString` _output_get)))

(fn `GenerateDamage`
  (params (damage :type Integer))
  (bind _output_get (set `self.CurrentHealth` (- (`self.CurrentHealth`) damage)))
  (if (< (`KismetMathLibrary.Conv_IntToDouble` _output_get) 0.1)
    (`self.K2_DestroyActor`)
    (else
      (bind _returnvalue (* (/ (`KismetMathLibrary.Conv_IntToDouble` _output_get) (`KismetMathLibrary.Conv_IntToDouble` (`self.InitialHealth`))) 100.0))
      (bind _output_get_2 (set `self.CurrentPercent` _returnvalue))))
  (`KismetSystemLibrary.PrintString` (`KismetStringLibrary.Conv_DoubleToString` _returnvalue) true true (struct :`R` 1.0 :`G` 0.015401 :`A` 1.0) 10.0))

(fn `UserConstructionScript`)