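; GM_TurnBased alternates turns between the player and an enemy, polling the turn state every Tick.
; The player's turn ends when BP_Player's AttackPoints drop below one, and the BP_UI widget shows whose turn it is.
; The enemy turn disables the UI, waits behind a re-entry flag, deals random damage, then restores attack points and control.
; The temporary damage text rolls its number separately from the damage dealt.
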(event `self.ReceiveTick`
  (params (DeltaSeconds :type "Float (single-precision)"))
  (`self.Turn Manager`))

(event `self.ReceiveBeginPlay`
  (bind _returnvalue (`GameplayStatics.GetActorOfClass` "/Game/Blueprints/Player/BP_Player.BP_Player_C"))
  (set `self.PlayerReference` _returnvalue)
  (bind _returnvalue_2 (`|CreateWidget` "/Game/Blueprints/UI/BP_UI.BP_UI_C"))
  (bind _output_get (set `self.UIReference` _returnvalue_2))
  (`UserWidget.AddToPlayerScreen` _output_get 0))

(event `EnemyTurn`
  (bind _returnvalue (`KismetMathLibrary.RandomIntegerInRange` 15 20))
  (bind _uireference (`self.UIReference`))
  (bind _playerreference (`self.PlayerReference`))
  (if (not (`self.DelayActive`))
    (`Widget.SetIsEnabled` (`self.UIReference`) false)
    (set `self.DelayActive` true)
    (`KismetSystemLibrary.Delay` 5.0)
    (`|ExecutionSequence`
      (:`then_0`
        (message `/Game/Blueprints/Utility/BPI_Damage.GenerateDamage` _playerreference _returnvalue)
        (set `self.IsPlayerTurn` true)
        (set `/Game/Blueprints/Player/BP_Player.AttackPoints` 3 _playerreference)
        (`Widget.SetIsEnabled` (`self.UIReference`) true)
        (set `self.DelayActive` false))
      (:`then_1`
        (`/Game/Blueprints/UI/BP_UI.SetTextDamageTaken` _uireference (`KismetTextLibrary.Conv_StringToText` (`KismetStringLibrary.Concat_StrStr` "You took " (`KismetStringLibrary.Conv_IntToString` _returnvalue) " damge")))
        (`KismetSystemLibrary.Delay` 3.0)
        (`/Game/Blueprints/UI/BP_UI.SetTextDamageTaken` _uireference "")))))

(fn `Player Turn`
  (bind _output_get (set `self.STR_Turn` "Your Turn!"))
  (`/Game/Blueprints/UI/BP_UI.SetTurnText` (`self.UIReference`) _output_get)
  (bind _returnvalue (`GameplayStatics.GetActorOfClass` "/Game/Blueprints/Player/BP_Player.BP_Player_C"))
  (if (< (`/Game/Blueprints/Player/BP_Player.AttackPoints` _returnvalue) 1)
    (set `self.IsPlayerTurn` false)
    (else
      (set `self.IsPlayerTurn` true))))

(fn `Turn Manager`
  (if (`self.IsPlayerTurn`)
    (`self.Player Turn`)
    (else
      (bind _output_get (set `self.STR_Turn` "Enemy's Turn!"))
      (`/Game/Blueprints/UI/BP_UI.SetTurnText` (`self.UIReference`) _output_get)
      (`self.EnemyTurn`))))

(fn `UserConstructionScript`)