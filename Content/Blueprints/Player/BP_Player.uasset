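; BP_Player is the player Blueprint that tracks health and shows it on a health UI widget.
; On BeginPlay it resets health to its initial values, prints debug values, and adds a BP_PlayerHealthUI widget to the player screen.
; GenerateDamage subtracts damage, then either destroys the actor when health drops below 0.1 or pushes the new health fraction to the widget.
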(event `self.ReceiveBeginPlay`
  (`KismetSystemLibrary.PrintString` (`KismetStringLibrary.Conv_IntToString` (`self.AttackPoints`)) true true (struct :`R` 0.090404 :`G` 0.240329 :`B` 1.0 :`A` 1.0))
  (set `self.CurrentHealth` (`self.InitialHealth`))
  (bind _output_get (set `self.CurrentPercent` (`self.InitialPercent`)))
  (`KismetSystemLibrary.PrintString` (`KismetStringLibrary.Conv_DoubleToString` _output_get))
  (bind _returnvalue (`|CreateWidget` "/Game/Blueprints/UI/BP_PlayerHealthUI.BP_PlayerHealthUI_C"))
  (bind _output_get_2 (set `self.PlayerHealth UI Reference` _returnvalue))
  (`UserWidget.AddToPlayerScreen` _output_get_2 0)
  (`/Game/Blueprints/UI/BP_PlayerHealthUI.SetPlayerHealth` (`self.PlayerHealth UI Reference`) _output_get))

(event `/Game/Blueprints/Utility/BPI_Damage.GenerateDamage`
  (params (DamageAmount :type Integer))
  (bind _output_get (set `self.CurrentHealth` (- (`self.CurrentHealth`) DamageAmount)))
  (if (< (`KismetMathLibrary.Conv_IntToDouble` _output_get) 0.1)
    (`self.K2_DestroyActor`)
    (else
      (bind _output_get_2 (set `self.CurrentPercent` (/ (`KismetMathLibrary.Conv_IntToDouble` _output_get) (`KismetMathLibrary.Conv_IntToDouble` (`self.InitialHealth`)))))
      (`/Game/Blueprints/UI/BP_PlayerHealthUI.SetPlayerHealth` (`self.PlayerHealth UI Reference`) _output_get_2))))

(fn `UserConstructionScript`)